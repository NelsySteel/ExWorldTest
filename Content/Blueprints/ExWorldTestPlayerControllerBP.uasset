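; Player controller for ExWorldTest that toggles a settings menu and manages persistent sound settings.
; On BeginPlay it creates the menu widget, loads settings from a save slot (or defaults), applies them, and starts background and music cues.
; ToggleMenu shows or hides the menu, switching cursor and input mode.
; SetSoundSettings applies per-category volumes as sound mix class overrides plus mute-when-unfocused; SaveSoundSettings writes them to the slot.
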(event EventBeginPlay
  (bind _returnvalue (UserInterface|CreateWidget "/Game/ThirdPerson/UI/Settings/SettingsMenuWidget.SettingsMenuWidget_C" (Game|GetPlayerController 0)))
  (Variables|Default|SetMenuWidget _returnvalue)
  (bind _soundsettings (CallFunction|LoadSoundSettings))
  (CallFunction|SetSoundSettings _soundsettings)
  (Audio|PlaySound2D "/Game/StarterContent/Audio/Starter_Background_Cue.Starter_Background_Cue" 1.0 1.0 0.0 0 0)
  (Audio|PlaySound2D "/Game/StarterContent/Audio/Starter_Music_Cue.Starter_Music_Cue" 1.0 1.0 0.0 0 0))

(event EventTick
  (params (DeltaSeconds :type Float%20%28single-precision%29)))

(event Input|ActionEvents|InputActionToggleMenu
  (params (Key :type Key%20Structure))
  (bind _menuwidget (Variables|Default|GetMenuWidget))
  (:Pressed
    (if (Variables|Default|GetMenuShown)
      (Widget|RemovefromParent _menuwidget)
      (Variables|Default|SetbShowMouseCursor false)
      (Input|SetInputModeGameandUI (Game|GetPlayerController 0) 0 "LockAlways" true)
      (else
        (UserInterface|Viewport|AddtoViewport _menuwidget 0)
        (Variables|Default|SetbShowMouseCursor true)
        (Input|SetInputModeGameandUI (Game|GetPlayerController 0) (Variables|Default|GetMenuWidget) "DoNotLock" false)))
    (Variables|Default|SetMenuShown (not (Variables|Default|GetMenuShown)))))

(fn ConstructionScript)

(fn LoadSoundSettings
  (bind _returnvalue (SaveGame|DoesSaveGameExist (Variables|Default|GetSoundSettingsSlot)))
  (if _returnvalue
    (bind _returnvalue_2 (SaveGame|LoadGamefromSlot (Variables|Default|GetSoundSettingsSlot)))
    (bind _assound_settings_save (Utilities|Casting|CastToSoundSettingsSave _returnvalue_2))
    (return (Variables|/Game/ThirdPerson/Sounds/SoundSettingsSave.SoundSettingsSave_C|GetSoundSettings _assound_settings_save))
    (else
      (return (Utilities|Struct|MakeSoundSettings 1.0 1.0)))))

(fn SaveSoundSettings
  (params (SoundSettings :type Sound%20Settings%20Structure))
  (bind _returnvalue (SaveGame|CreateSaveGameObject "/Game/ThirdPerson/Sounds/SoundSettingsSave.SoundSettingsSave_C"))
  (Variables|/Game/ThirdPerson/Sounds/SoundSettingsSave.SoundSettingsSave_C|SetSoundSettings _returnvalue SoundSettings)
  (SaveGame|SaveGametoSlot _returnvalue (Variables|Default|GetSoundSettingsSlot)))

(fn SetSoundSettings
  (params (SoundSettings :type Sound%20Settings%20Structure))
  (Utilities|FlowControl|Sequence
    (:then_0
      (Audio|SetSoundMixClassOverride "/Game/ThirdPerson/Sounds/SoundClasses/ExWorldTestSoundMixModifier.ExWorldTestSoundMixModifier" "/Game/ThirdPerson/Sounds/SoundClasses/ExWorldTestMaster.ExWorldTestMaster" (.mastervolume SoundSettings) 1.0 0.0 true))
    (:then_1
      (Audio|SetSoundMixClassOverride "/Game/ThirdPerson/Sounds/SoundClasses/ExWorldTestSoundMixModifier.ExWorldTestSoundMixModifier" "/Game/ThirdPerson/Sounds/SoundClasses/ExWorldTestSFX.ExWorldTestSFX" (.sfxvolume SoundSettings) 1.0 0.0 true))
    (:then_2
      (Audio|SetSoundMixClassOverride "/Game/ThirdPerson/Sounds/SoundClasses/ExWorldTestSoundMixModifier.ExWorldTestSoundMixModifier" "/Game/ThirdPerson/Sounds/SoundClasses/ExWorldTestMusic.ExWorldTestMusic" (.musicvolume SoundSettings) 1.0 0.0 true))
    (:then_3
      (Audio|SetSoundMixClassOverride "/Game/ThirdPerson/Sounds/SoundClasses/ExWorldTestSoundMixModifier.ExWorldTestSoundMixModifier" "/Game/ThirdPerson/Sounds/SoundClasses/ExWorldTestBackground.ExWorldTestBackground" (.backgroundsoundsvolume SoundSettings) 1.0 0.0 true))
    (:then_4
      (Audio|SetSoundMixClassOverride "/Game/ThirdPerson/Sounds/SoundClasses/ExWorldTestSoundMixModifier.ExWorldTestSoundMixModifier" "/Game/ThirdPerson/Sounds/SoundClasses/ExWorldTestCinematics.ExWorldTestCinematics" (.cinematicsvolume SoundSettings) 1.0 0.0 true))
    (:then_5
      (Audio|SetSoundMixClassOverride "/Game/ThirdPerson/Sounds/SoundClasses/ExWorldTestSoundMixModifier.ExWorldTestSoundMixModifier" "/Game/ThirdPerson/Sounds/SoundClasses/ExWorldTestUISounds.ExWorldTestUISounds" (.uisoundsvolume SoundSettings) 1.0 0.0 true))
    (:then_6
      (Audio|SetSoundMixClassOverride "/Game/ThirdPerson/Sounds/SoundClasses/ExWorldTestSoundMixModifier.ExWorldTestSoundMixModifier" "/Game/ThirdPerson/Sounds/SoundClasses/ExWorldTestNPCVoices.ExWorldTestNPCVoices" (.voicesvolume SoundSettings) 1.0 0.0 true))
    (:then_7
      (Audio|SetSoundMixClassOverride "/Game/ThirdPerson/Sounds/SoundClasses/ExWorldTestSoundMixModifier.ExWorldTestSoundMixModifier" "/Game/ThirdPerson/Sounds/SoundClasses/ExWorldTestBackgroundVoices.ExWorldTestBackgroundVoices" (.backgroundvoicesvolume SoundSettings) 1.0 0.0 true))
    (:then_8
      (Audio|SetSoundMixClassOverride "/Game/ThirdPerson/Sounds/SoundClasses/ExWorldTestSoundMixModifier.ExWorldTestSoundMixModifier" "/Game/ThirdPerson/Sounds/SoundClasses/ExWorldTestDialogs.ExWorldTestDialogs" (.dialogsvolume SoundSettings) 1.0 0.0 true))
    (:then_9
      (Class|SoundsBlueprintFunctionLibrary|SetUnfocusedVolumeMuted (.muteunfocused SoundSettings)))
    (:then_10
      (Audio|SetSoundMixClassOverride "/Game/ThirdPerson/Sounds/SoundClasses/ExWorldTestSoundMixModifier.ExWorldTestSoundMixModifier" "/Game/ThirdPerson/Sounds/SoundClasses/ExWorldTestPlayerVoice.ExWorldTestPlayerVoice" (.microhonelevel SoundSettings) 1.0 0.0 true))))